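; BP_TestActor is a test interactable that registers itself with the player controller while the player is within reach.
; Its Sphere overlap events compare the other actor's class to the player pawn's, then update InReach and LastInteractedActor on PlayerControlling.
; Entering and leaving both toggle the ActionButton's visibility.
; PossessAction, not called within this Blueprint, swaps the mesh material to RedPossess.
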(event `self.Sphere.OnComponentBeginOverlap`
  (params (OverlappedComponent :type "PrimitiveComponent Object Reference") (OtherActor :type "Actor Object Reference") (OtherComp :type "PrimitiveComponent Object Reference") (OtherBodyIndex :type Integer) (bFromSweep :type Boolean) (SweepResult :type "HitResult Structure (by ref)"))
  (if (== (`GameplayStatics.GetObjectClass` (`GameplayStatics.GetPlayerPawn` 0)) (`GameplayStatics.GetObjectClass` OtherActor))
    (set `self.InReach` true)
    (bind _asplayer_controlling (cast `/Game/ThirdPersonBP/Blueprints/PlayerControlling` (`GameplayStatics.GetPlayerController` 0)))
    (set `/Game/ThirdPersonBP/Blueprints/PlayerControlling.LastInteractedActor` self _asplayer_controlling)
    (set `/Game/ThirdPersonBP/Blueprints/PlayerControlling.InReach` (`self.InReach`) _asplayer_controlling :!label _label)
    (`SceneComponent.ToggleVisibility` (`self.ActionButton`) false)))

(event `self.Sphere.OnComponentEndOverlap`
  (params (OverlappedComponent :type "PrimitiveComponent Object Reference") (OtherActor :type "Actor Object Reference") (OtherComp :type "PrimitiveComponent Object Reference") (OtherBodyIndex :type Integer))
  (if (== (`GameplayStatics.GetObjectClass` (`GameplayStatics.GetPlayerPawn` 0)) (`GameplayStatics.GetObjectClass` OtherActor))
    (set `self.InReach` false)
    (bind _asplayer_controlling (cast `/Game/ThirdPersonBP/Blueprints/PlayerControlling` (`GameplayStatics.GetPlayerController` 0)))
    (set `/Game/ThirdPersonBP/Blueprints/PlayerControlling.LastInteractedActor` null _asplayer_controlling)
    (goto _label)))

(fn `PossessAction`
  (`PrimitiveComponent.SetMaterial` (`self.Mesh`) 0 "/Game/Shaders/Material/RedPossess.RedPossess"))

(fn `UserConstructionScript`)
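; Test pawn for a side-offset camera, with a cube mesh that switches to a blue material on its possess event.
; Turn and LookUp axes add controller yaw and pitch, provided player controller 0 is a PlayerControlling.
; Both axes then share one step that adds the side offset's Z to BaseCamera's current world yaw, keeping pitch and roll.
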(event `InputAxis|Turn`
  (params (AxisValue :type "Float (single-precision)"))
  (bind _basecamera (`self.BaseCamera`))
  (bind (_vcamerasideoffset_x _vcamerasideoffset_y _vcamerasideoffset_z) (`KismetMathLibrary.BreakVector` (`self.vCameraSideOffset`)))
  (bind (_returnvalue_roll _returnvalue_pitch _returnvalue_yaw) (`KismetMathLibrary.BreakRotator` (`SceneComponent.K2_GetComponentRotation` _basecamera)))
  (cast `/Game/ThirdPersonBP/Blueprints/PlayerControlling` (`GameplayStatics.GetPlayerController` 0))
  (`self.AddControllerYawInput` AxisValue)
  (`SceneComponent.K2_SetWorldRotation` _basecamera (`KismetMathLibrary.MakeRotator` _returnvalue_roll _returnvalue_pitch (+ _returnvalue_yaw _vcamerasideoffset_z)) false false :!label _label))

(event `InputAxis|LookUp`
  (params (AxisValue :type "Float (single-precision)"))
  (cast `/Game/ThirdPersonBP/Blueprints/PlayerControlling` (`GameplayStatics.GetPlayerController` 0))
  (`self.AddControllerPitchInput` AxisValue)
  (goto _label))

(event `self.PossessAction`
  (`PrimitiveComponent.SetMaterial` (`self.CubeMesh`) 0 "/Game/Shaders/Material/BluePossess.BluePossess"))

(fn `UserConstructionScript`
  (`parent.UserConstructionScript`))